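; A trigger volume that damages the player's 2D side-scroller character while it overlaps the Box.
; Each Tick, CheckTrigger polls the Box for player pawn 0, and DamageMode selects the behavior through DoOnce gates.
; DOT hits on entry and again whenever a delta-time timer reaches DOTDamageInterval, while Once hits a single time per entry.
; Leaving the box re-arms the gate, so re-entry deals damage immediately.
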(event EventBeginPlay)

(event Collision|EventActorBeginOverlap
  (params (OtherActor :type Actor%20Object%20Reference)))

(event EventTick
  (params (DeltaSeconds :type Float%20%28single-precision%29))
  (switch Utilities|FlowControl|Switch|SwitchonVolumeDamage (Variables|Default|GetDamageMode)
    (:NewEnumerator0
      (Utilities|FlowControl|Sequence
        (:then_0
          (bind _ischarinside (CallFunction|CheckTrigger (Variables|Default|GetBox)))
          (if _ischarinside
            (Utilities|FlowControl|DoOnce false :!label _label
              (:Completed
                (bind _as2dside_scroller_character (Utilities|Casting|CastTo2DSideScrollerCharacter (Game|Player|GetPlayerPawn 0)))
                (Default|TakeDamage _as2dside_scroller_character (Variables|Default|GetDamageValue))
                (Variables|Default|Settimer 0.0)))
            (else
              (goto _label Reset))))
        (:then_1
          (bind _output_get (Variables|Default|Settimer (+ (Variables|Default|Gettimer) (Utilities|Time|GetWorldDeltaSeconds))))
          (if (>= _output_get (Variables|Default|GetDOTDamageInterval))
            (goto _label Reset)))))
    (:NewEnumerator1
      (bind _ischarinside_2 (CallFunction|CheckTrigger (Variables|Default|GetBox)))
      (if _ischarinside_2
        (Utilities|FlowControl|DoOnce false :!label _label_2
          (:Completed
            (bind _as2dside_scroller_character_2 (Utilities|Casting|CastTo2DSideScrollerCharacter (Game|Player|GetPlayerPawn 0)))
            (Default|TakeDamage _as2dside_scroller_character_2 (Variables|Default|GetDamageValue))))
        (else
          (goto _label_2 Reset))))))

(fn ConstructionScript)

(fn CheckTrigger
  (params (box :type Box%20Component%20Object%20Reference))
  (if (Utilities|Array|ContainsItem (Collision|GetOverlappingActors box "/Game/Characters/Hero/2DSideScrollerCharacter.2DSideScrollerCharacter_C" :!class /Script/Engine.PrimitiveComponent) (Game|Player|GetPlayerPawn 0))
    (return true)
    (else
      (return false))))