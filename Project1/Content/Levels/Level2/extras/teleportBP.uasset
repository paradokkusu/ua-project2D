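; Level 2 teleporter Blueprint that moves the player pawn to a Location when it stands inside the Box volume.
; Each Tick, CheckTrigger tests whether player pawn 0 is among the Box's overlapping actors.
; While it is, the pawn is set to that Location without sweep or physics teleport, polling rather than using overlap events.
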(event EventBeginPlay)

(event Collision|EventActorBeginOverlap
  (params (OtherActor :type Actor%20Object%20Reference)))

(event EventTick
  (params (DeltaSeconds :type Float%20%28single-precision%29))
  (bind _hit (CallFunction|CheckTrigger (Variables|Default|GetBox)))
  (if _hit
    (Transformation|SetActorLocation (Game|Player|GetPlayerPawn 0) (Variables|Default|Getlocation) false false)))

(fn ConstructionScript)

(fn CheckTrigger
  (params (box :type Box%20Component%20Object%20Reference))
  (if (Utilities|Array|ContainsItem (Collision|GetOverlappingActors box 0 :!class /Script/Engine.PrimitiveComponent) (Game|Player|GetPlayerPawn 0))
    (return true)
    (else
      (return false))))