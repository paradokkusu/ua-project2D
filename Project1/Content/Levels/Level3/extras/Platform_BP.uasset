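; Moving platform actor for a level that travels back and forth along the world X and Z axes.
; BeginPlay stores the start location, then each Tick offsets the position by per-axis speed, direction and delta time.
; Separate bound checks update each axis direction whenever the platform leaves the range between its start and start plus that axis's distance.
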(event EventBeginPlay
  (Variables|Default|SetinitPosition (Transformation|GetActorLocation)))

(event Collision|EventActorBeginOverlap
  (params (OtherActor :type Actor%20Object%20Reference)))

(event EventTick
  (params (DeltaSeconds :type Float%20%28single-precision%29))
  (CallFunction|UpdatePlatformPos)
  (CallFunction|CheckBoundX)
  (CallFunction|CheckBoundZ))

(fn ConstructionScript)

(fn UpdatePlatformPos
  (bind _returnvalue (Transformation|GetActorLocation))
  (Transformation|SetActorLocation (Math|Vector|MakeVector (+ (* (Variables|Default|GetspeedX) (Utilities|Time|GetWorldDeltaSeconds) (Variables|Default|GetdirectionX)) (.x _returnvalue)) (.y _returnvalue) (+ (.z _returnvalue) (* (Utilities|Time|GetWorldDeltaSeconds) (Variables|Default|GetdirectionZ) (Variables|Default|GetspeedZ)))) false false))

(fn CheckBoundX
  (bind _returnvalue (Transformation|GetActorLocation))
  (bind _initposition (Variables|Default|GetinitPosition))
  (if (or (> (.x _returnvalue) (+ (.x _initposition) (Variables|Default|GetdistanceX))) (< (.x _returnvalue) (.x _initposition)))
    (bind _result (Math|Float|NegateFloat (Variables|Default|GetdirectionX))
      (:%20%20
        (Variables|Default|SetdirectionX _result)))))

(fn CheckBoundZ
  (bind _returnvalue (Transformation|GetActorLocation))
  (bind _initposition (Variables|Default|GetinitPosition))
  (if (or (> (.z _returnvalue) (+ (.z _initposition) (Variables|Default|GetdistanceZ))) (< (.z _returnvalue) (.z _initposition)))
    (bind _result (Math|Float|NegateFloat (Variables|Default|GetdirectionZ))
      (:%20%20
        (Variables|Default|SetdirectionZ _result)))))