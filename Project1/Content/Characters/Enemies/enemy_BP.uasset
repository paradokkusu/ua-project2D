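; Paper2D side-scroller enemy that patrols platforms and attacks the hero, with stats and flipbooks looked up in maps by enemy type.
; Tick prioritises death, hurt, attack, then patrol, using two downward edge traces to turn at ledges.
; A sphere trace detects characters; after the attack flipbook finishes, it spawns a melee damage actor or projectile and starts a cooldown.
; Overlapping MeleeDamage_BP costs one health, and death destroys the actor after its animation.
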(event OnComponentBeginOverlap(Box)
  (params (OverlappedComponent :type Primitive%20Component%20Object%20Reference) (OtherActor :type Actor%20Object%20Reference) (OtherComp :type Primitive%20Component%20Object%20Reference) (OtherBodyIndex :type Integer) (bFromSweep :type Boolean) (SweepResult :type Hit%20Result%20Structure%20%28by%20ref%29))
  ;[1 1 1] Take damage
  (if (== (Utilities|GetClass OtherActor) "/Game/Characters/MeleeDamage_BP.MeleeDamage_BP_C")
    (CallFunction|TakeDamage 1)))

(event Custom|UpdateHurt
  (bind _mainfb (Variables|Default|GetMainFB))
  ;[1 1 1] Update Hurt
  (bind _flipbook (Flipbooks|GetFBHurt))
  (Sprite|SetFlipbook (Variables|Default|GetMainFB) _flipbook)
  (if (== (+ (Class|PaperFlipbookComponent|GetPlaybackPositioninFrames _mainfb) 1) (Class|PaperFlipbookComponent|GetFlipbookLengthinFrames _mainfb))
    (Variables|Default|SetisHurt false)))

(event Custom|HandleDeath
  (bind _mainfb (Variables|Default|GetMainFB))
  ;[1 1 1] Handle death
  (bind _flipbook (Flipbooks|GetFBDeath))
  (Sprite|SetFlipbook (Variables|Default|GetMainFB) _flipbook)
  (if (== (+ (Class|PaperFlipbookComponent|GetPlaybackPositioninFrames _mainfb) 1) (Class|PaperFlipbookComponent|GetFlipbookLengthinFrames _mainfb))
    (Actor|DestroyActor)))

(event Custom|UpdateAttack
  (bind _mainfb (Variables|Default|GetMainFB))
  ;[1 1 1] Handle Attack
  (bind _flipbook (Flipbooks|GetFBAttack))
  (Sprite|SetFlipbook (Variables|Default|GetMainFB) _flipbook)
  (if (== (+ (Class|PaperFlipbookComponent|GetPlaybackPositioninFrames _mainfb) 1) (Class|PaperFlipbookComponent|GetFlipbookLengthinFrames _mainfb))
    (Variables|Default|SetattackEnd true)))

(event EventBeginPlay
  (bind _enemy (Variables|Default|Getenemy))
  (bind _returnvalue (Utilities|String|EnumtoString _enemy))
  (bind _output_get (Variables|Default|SetmaxHealth (.Value (Utilities|Map|Find (Variables|Default|GetattackNumber) _returnvalue))))
  (Variables|Default|SetcurrentHealth _output_get)
  (Variables|Default|Setspeed (.Value (Utilities|Map|Find (Variables|Default|GetspeedMap) _returnvalue)))
  (Variables|Default|SetcoolDown (.Value (Utilities|Map|Find (Variables|Default|GetattackCooldownMap) _returnvalue)))
  (switch Utilities|FlowControl|Switch|SwitchonAttackType (Variables|Default|GetattackType)
    (:NewEnumerator0
      (Variables|Default|SetdetectionRadius 6e+01))
    (:NewEnumerator1
      (Variables|Default|SetdetectionRadius 2e+02))))

(event Collision|EventActorBeginOverlap
  (params (OtherActor :type Actor%20Object%20Reference)))

(event EventTick
  (params (DeltaSeconds :type Float%20%28single-precision%29))
  (Utilities|FlowControl|Sequence
    (:then_0
      (if (> (Variables|Default|GetcooldownTimer) 0.0)
        (Variables|Default|SetcooldownTimer (- (Variables|Default|GetcooldownTimer) (Utilities|Time|GetWorldDeltaSeconds)))
        (else
          (Variables|Default|SetcooldownTimer 0.0)
          (goto _label Reset))))
    (:then_1
      (if (<= (Variables|Default|GetcurrentHealth) 0)
        (CallFunction|HandleDeath)
        (elif (Variables|Default|GetisHurt)
          (CallFunction|UpdateHurt)
          (else
            (bind _hit (CallFunction|CheckDetection (Variables|Default|GetdetectionRadius)))
            (if _hit
              (CallFunction|FaceHero)
              (if (== (Variables|Default|GetcooldownTimer) 0.0)
                (if (Variables|Default|GetattackEnd)
                  (Utilities|FlowControl|DoOnce false :!label _label
                    (:Completed
                      (Variables|Default|SetcooldownTimer (Variables|Default|GetcoolDown))
                      (if (Utilities|Enum|Equal(Enum) (Variables|Default|GetattackType) "NewEnumerator0")
                        (Game|SpawnActorfromClass "/Game/Characters/HeroDamage_BP.HeroDamage_BP_C" (Transformation|GetWorldTransform (Variables|Default|GetArrow)) "Undefined" 0 0)
                        (Variables|Default|SetattackEnd false)
                        (else
                          (Game|SpawnActorfromClass (.Value (Utilities|Map|Find (Variables|Default|GetprojectileClass) (Utilities|String|EnumtoString (Variables|Default|GetprojectileType)))) (Math|Transform|MakeTransform (Transformation|GetActorLocation) "0, 0, 0" "1,1,1") "Undefined" 0 0)
                          (Variables|Default|SetattackEnd false)))))
                  (else
                    (CallFunction|UpdateAttack)))
                (else
                  (bind _flipbook (Flipbooks|GetFBIdle))
                  (Sprite|SetFlipbook (Variables|Default|GetMainFB) _flipbook)))
              (else
                (Variables|Default|SetcooldownTimer 0.0)
                (bind _axisout (CallFunction|RaycastGround))
                (CallFunction|Movement _axisout (Variables|Default|Getspeed))))))))))

(fn ConstructionScript)

(fn CheckDetection
  (params (Distance :type Float%20%28single-precision%29))
  (bind _returnvalue (Transformation|GetActorLocation))
  (bind _outhits (Collision|MultiSphereTraceByChannel _returnvalue _returnvalue Distance "TraceTypeQuery1" false 0 "ForOneFrame" true "(R=1.000000,G=0.000000,B=0.000000,A=1.000000)" "(R=0.000000,G=1.000000,B=0.000000,A=1.000000)" 1.0))
  (for _array_element _outhits
    (Utilities|Casting|CastToPaperCharacter (.HitActor (Collision|BreakHitResult _array_element)))
    (return true))
  (return false))

(fn RaycastGround
  (bind _box (Variables|Default|GetBox))
  (bind _box_2 (Variables|Default|GetBox))
  (bind (_origin _boxextent) (Collision|GetComponentBounds _box))
  (bind (_origin_2 _boxextent_2) (Collision|GetComponentBounds _box_2))
  (bind _returnvalue (- (.z _origin_2) (.z _boxextent_2)))
  (bind _returnvalue_2 (- (.x _origin_2) (.x _boxextent_2)))
  (bind _returnvalue_3 (- (.z _origin) (.z _boxextent)))
  (bind _returnvalue_4 (+ (.x _origin) (.x _boxextent)))
  (bind _returnvalue_5 (Collision|LineTraceByChannel (Math|Vector|MakeVector _returnvalue_2 (.y _origin_2) (- _returnvalue 2.0)) (Math|Vector|MakeVector _returnvalue_2 (.y _origin_2) (- _returnvalue 1e+01)) "TraceTypeQuery1" false 0 "ForOneFrame" true "(R=1.000000,G=0.000000,B=0.000000,A=1.000000)" "(R=0.000000,G=1.000000,B=0.000000,A=1.000000)" 1.0))
  (if (not _returnvalue_5)
    (bind _output_get (Variables|Default|SetwalkAxis 1.0))
    (return _output_get)
    (else
      (bind _returnvalue_6 (Collision|LineTraceByChannel (Math|Vector|MakeVector _returnvalue_4 (.y _origin) _returnvalue_3) (Math|Vector|MakeVector _returnvalue_4 (.y _origin) (- _returnvalue_3 1e+01)) "TraceTypeQuery1" false 0 "ForOneFrame" true "(R=1.000000,G=0.000000,B=0.000000,A=1.000000)" "(R=0.000000,G=1.000000,B=0.000000,A=1.000000)" 1.0))
      (if (not _returnvalue_6)
        (bind _output_get_2 (Variables|Default|SetwalkAxis -1.0))
        (return _output_get_2)
        (else
          (return (Variables|Default|GetwalkAxis)))))))

(fn Movement
  (params (AxisIN :type Float%20%28single-precision%29) (SpeedIN :type Float%20%28single-precision%29))
  (bind _returnvalue (Transformation|GetActorLocation))
  (if (== AxisIN 1.0)
    ;[0.9952 1 0.4496] Flipbook Animation logic to reverse based on location
    (Transformation|ResetRelativeTransform (Variables|Default|GetMainFB))
    (bind _flipbook (Flipbooks|GetFBWalk))
    (Sprite|SetFlipbook (Variables|Default|GetMainFB) _flipbook)
    (else
      (bind _flipbook_2 (Flipbooks|GetFBWalk))
      (Sprite|SetFlipbook (Variables|Default|GetMainFB) _flipbook_2)
      (Transformation|SetRelativeRotation (Variables|Default|GetMainFB) (Math|Rotator|MakeRotator 0.0 0.0 1.8e+02) false false)))
  (Transformation|SetActorLocation (Math|Vector|MakeVector (+ (* AxisIN SpeedIN (Utilities|Time|GetWorldDeltaSeconds)) (.x _returnvalue)) (.y _returnvalue) (.z _returnvalue)) false false))

(fn TakeDamage
  (params (damage :type Integer))
  (if (< damage (Variables|Default|GetcurrentHealth))
    (bind _output_get (Variables|Default|SetcurrentHealth (- (Variables|Default|GetcurrentHealth) damage)))
    (Variables|Default|SetisHurt true)
    (Development|PrintString (Utilities|String|ToString(Integer) _output_get))
    (else
      (Variables|Default|SetcurrentHealth 0))))

(fn FaceHero
  (Utilities|FlowControl|Sequence
    (:then_0
      (bind _as2dside_scroller_character (Utilities|Casting|CastTo2DSideScrollerCharacter (Game|GetPlayerCharacter 0)))
      (if (and (> (.x (Transformation|GetActorLocation _as2dside_scroller_character)) (.x (Transformation|GetActorLocation))) (== (Variables|Default|GetwalkAxis) -1.0))
        (Transformation|ResetRelativeTransform (Variables|Default|GetMainFB))
        (bind _flipbook (Flipbooks|GetFBWalk))
        (Sprite|SetFlipbook (Variables|Default|GetMainFB) _flipbook)
        (Variables|Default|SetwalkAxis 1.0)))
    (:then_1
      (bind _as2dside_scroller_character_2 (Utilities|Casting|CastTo2DSideScrollerCharacter (Game|GetPlayerCharacter 0)))
      (if (and (> (.x (Transformation|GetActorLocation)) (.x (Transformation|GetActorLocation _as2dside_scroller_character_2))) (== (Variables|Default|GetwalkAxis) 1.0))
        (bind _flipbook_2 (Flipbooks|GetFBWalk))
        (Sprite|SetFlipbook (Variables|Default|GetMainFB) _flipbook_2)
        (Transformation|SetRelativeRotation (Variables|Default|GetMainFB) (Math|Rotator|MakeRotator 0.0 0.0 1.8e+02) false false)
        (Variables|Default|SetwalkAxis -1.0)))))

(fn GetFBIdle
  (return (.Value (Utilities|Map|Find (Variables|Flipbooks|GetIdleFB) (Utilities|String|EnumtoString (Variables|Default|Getenemy))))))

(fn GetFBWalk
  (return (.Value (Utilities|Map|Find (Variables|Flipbooks|GetwalkFB) (Utilities|String|EnumtoString (Variables|Default|Getenemy))))))

(fn GetFBAttack
  (return (.Value (Utilities|Map|Find (Variables|Flipbooks|GetattackFB) (Utilities|String|EnumtoString (Variables|Default|Getenemy))))))

(fn GetFBHurt
  (return (.Value (Utilities|Map|Find (Variables|Flipbooks|GethurtFB) (Utilities|String|EnumtoString (Variables|Default|Getenemy))))))

(fn GetFBDeath
  (return (.Value (Utilities|Map|Find (Variables|Flipbooks|GetdeathFB) (Utilities|String|EnumtoString (Variables|Default|Getenemy))))))