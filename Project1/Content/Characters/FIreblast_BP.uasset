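; Fireblast is a flipbook-animated projectile for a 2D side-scroller, aimed at the player's position when it spawns.
; BeginPlay caches direction and look-at rotation, so it does not home afterwards.
; In Linear shoot mode, Tick plays a timeline whose track scales Speed, moving the actor without sweep on each update.
; It destroys itself on the flipbook's last frame or shortly after overlapping the player character, applying no damage here.
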(event OnComponentBeginOverlap(Box)
  (params (OverlappedComponent :type Primitive%20Component%20Object%20Reference) (OtherActor :type Actor%20Object%20Reference) (OtherComp :type Primitive%20Component%20Object%20Reference) (OtherBodyIndex :type Integer) (bFromSweep :type Boolean) (SweepResult :type Hit%20Result%20Structure%20%28by%20ref%29))
  (if (== (Utilities|GetClass OtherActor) "/Game/Characters/Hero/2DSideScrollerCharacter.2DSideScrollerCharacter_C")
    (Utilities|FlowControl|Delay 0.2)
    (Actor|DestroyActor)))

(event EventBeginPlay
  (bind (_direction _rotation) (CallFunction|DirectionandRotation))
  (Variables|Default|SetDirection _direction)
  (Variables|Default|SetProjectileRotation _rotation))

(event Collision|EventActorBeginOverlap
  (params (OtherActor :type Actor%20Object%20Reference)))

(event EventTick
  (params (DeltaSeconds :type Float%20%28single-precision%29))
  (switch Utilities|FlowControl|Switch|SwitchonShootMode (Variables|Default|GetShootMode)
    (:NewEnumerator0
      (bind _newtrack_0 (Timeline|TimelineProjectile Play)
        (:Update
          (CallFunction|MovingProjectile (Variables|Default|GetProjectileRotation) (Variables|Default|GetDirection) (* _newtrack_0 (Variables|Default|GetSpeed))))))))

(fn ConstructionScript)

(fn MovingProjectile
  (params (Rotation :type Rotator) (Direction :type Vector) (Speed :type Float%20%28single-precision%29))
  (bind _returnvalue (Transformation|GetActorTransform))
  (bind _projectilefb (Variables|Default|GetProjectileFB))
  (Transformation|SetActorTransform (Math|Transform|MakeTransform (+ (* Direction (* (Utilities|Time|GetWorldDeltaSeconds) Speed)) (.location _returnvalue)) Rotation (.scale _returnvalue)))
  (if (== (+ (Class|PaperFlipbookComponent|GetPlaybackPositioninFrames _projectilefb) 1) (Class|PaperFlipbookComponent|GetFlipbookLengthinFrames _projectilefb))
    (Actor|DestroyActor)))

(fn DirectionandRotation
  (bind _returnvalue (Game|Player|GetPlayerPawn 0))
  (bind _returnvalue_2 (Transformation|GetActorLocation))
  (bind _returnvalue_3 (Transformation|GetActorLocation _returnvalue))
  (bind _returnvalue_4 (Math|Rotator|FindLookatRotation _returnvalue_2 _returnvalue_3))
  (return (Math|Vector|Normalize (- _returnvalue_3 _returnvalue_2)) (Math|Rotator|MakeRotator (.roll _returnvalue_4) (.pitch _returnvalue_4) (.yaw _returnvalue_4))))